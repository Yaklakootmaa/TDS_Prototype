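; BPC_DamageSystem is a component that gives its owner health, with events for taking damage (blocked when immortal) and healing capped at the maximum.
; At BeginPlay it fills health, starts a looping HealthCheck timer and caches the player via a message to the player controller.
; When health runs out, HealthCheck prints game over for the player; other owners send their score to the player and are destroyed.
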(event `self.ReceiveBeginPlay`
  (set `self.HealthCurrent` (`self.HealthMax`))
  (`KismetSystemLibrary.K2_SetTimerDelegate` (delegate `HealthCheck`) 0.1 true)
  (`KismetSystemLibrary.Delay` 0.0)
  (bind _player (message `/Game/BP_Interface/BPI_GameSystems.TriggerGetPlayer` (`GameplayStatics.GetPlayerController` 0)))
  (set `self.Player` _player))

(event `HealthCheck`
  (bind _player (`self.Player`))
  (if (<= (`self.HealthCurrent`) 0.0)
    (if (== (`self.GetOwner`) _player)
      (`KismetSystemLibrary.PrintString` "Player is dead - game over" true true (struct :`R` 1.0 :`G` 0.051901 :`A` 1.0))
      (else
        (message `/Game/BP_Interface/BPI_GameSystems.TriggerGiveScore` _player (`self.Score`))
        (`Actor.K2_DestroyActor` (`self.GetOwner`))))))

(event `/Game/BP_Interface/BPI_GameSystems.TriggerCauseDamage`
  (params (Damage :type "Float (double-precision)"))
  (if (`self.IsImmortal`)
    (`KismetSystemLibrary.PrintString` "IMMORTAL!" true true (struct :`R` 0.075611 :`G` 1.0 :`A` 1.0))
    (else
      (bind _output_get (set `self.HealthCurrent` (- (`self.HealthCurrent`) Damage)))
      (`KismetSystemLibrary.PrintString` (`KismetStringLibrary.Conv_DoubleToString` _output_get) true true (struct :`R` 1.0 :`G` 0.051901 :`A` 1.0)))))

(event `/Game/BP_Interface/BPI_GameSystems.TriggerAddHealth`
  (params (Health :type "Float (double-precision)"))
  (bind _returnvalue (+ (`self.HealthCurrent`) Health))
  (if (> _returnvalue (`self.HealthMax`))
    (set `self.HealthCurrent` (`self.HealthMax`))
    (else
      (set `self.HealthCurrent` _returnvalue)))
  (`KismetSystemLibrary.PrintString` (`KismetStringLibrary.Conv_DoubleToString` (`self.HealthCurrent`)) true true (struct :`R` 0.075611 :`G` 1.0 :`A` 1.0)))

(fn `TriggerGetPlayer`
  (returns (Player :type "Actor Object Reference"))
  (return null))

(fn `TriggerGetScore`
  (returns (Score :type "Float (double-precision)"))
  (return 0.0))