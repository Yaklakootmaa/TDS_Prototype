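; BP_Enemy is a simple melee enemy that chases the player and damages them at close range.
; On BeginPlay it finds BP_Player and starts two looping timers instead of using Tick.
; One timer refreshes an AI MoveTo toward the player's location.
; The other checks distance against MeleeDistance and triggers MeleeDamage through the player's BPC_DamageSystem component.
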(event `self.ReceiveBeginPlay`
  (bind _returnvalue (`GameplayStatics.GetActorOfClass` "/Game/BP_Player.BP_Player_C"))
  (set `self.PlayerPawn` _returnvalue)
  (`KismetSystemLibrary.K2_SetTimerDelegate` (delegate `UpdateTarget`) 0.25 true)
  (`KismetSystemLibrary.K2_SetTimerDelegate` (delegate `CauseMelee`) 0.5 true)
  (bind _returnvalue_2 (`GameplayStatics.GetActorOfClass` "/Game/BP_Player.BP_Player_C"))
  (set `self.Player` _returnvalue_2))

(event `CauseMelee`
  (if (<= (`KismetMathLibrary.Vector_Distance` (`self.K2_GetActorLocation` (`self.Player`)) (`self.K2_GetActorLocation`)) (`self.MeleeDistance`))
    (message `/Game/BP_Interface/BPI_GameSystems.TriggerCauseDamage` (`self.GetComponentByClass` (`self.Player`) "/Game/Component/BPC_DamageSystem.BPC_DamageSystem_C") (`self.MeleeDamage`))))

(event `UpdateTarget`
  (`AIController.MoveToLocation` (`AIBlueprintHelperLibrary.GetAIController` self) (`self.K2_GetActorLocation` (`self.PlayerPawn`)) -1.0 true true false true null true))

(fn `UserConstructionScript`)