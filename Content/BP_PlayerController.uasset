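; Player controller that relays Enhanced Input to the controlled pawn and exposes that pawn through a getter.
; When handed a pawn, it stores it, adds the input mapping context, then forwards movement, strafe, rotation, action and reload as messages.
; Action1 splits tap from hold by comparing triggered time against one dilation-corrected frame.
; Debug-style F1–F3 keys cast to BP_Player to switch graphics quality; the HUD info getter returns only empty defaults.
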(event `/Game/BP_Interface/BPI_Controls.TriggerGetPawnInfo`
  (params (Pawn :type "Actor Object Reference"))
  (bind _returnvalue (pcsubsystem `EnhancedInputLocalPlayerSubsystem` self))
  (set `self.PlayerPawn` Pawn)
  (`/Engine/EditorBlueprintResources/StandardMacros.IsValid` _returnvalue
    (:`Is Valid`
      (`EnhancedInputSubsystemInterface.AddMappingContext` _returnvalue "/Game/Input/IMC_PlayerInput.IMC_PlayerInput" 0 (struct)))))

(event `EnhancedInput|/Game/Input/IA_Movement`
  (params (ActionValue :type "Float (double-precision)") (ElapsedSeconds :type "Float (double-precision)") (TriggeredSeconds :type "Float (double-precision)") (InputAction :type "InputAction Object Reference" :default "/Game/Input/IA_Movement.IA_Movement"))
  (:`Triggered`
    (message `/Game/BP_Interface/BPI_Controls.TriggerSetMovement` (`self.PlayerPawn`) ActionValue)))

(event `EnhancedInput|/Game/Input/IA_Strafe`
  (params (ActionValue :type "Float (double-precision)") (ElapsedSeconds :type "Float (double-precision)") (TriggeredSeconds :type "Float (double-precision)") (InputAction :type "InputAction Object Reference" :default "/Game/Input/IA_Strafe.IA_Strafe"))
  (:`Triggered`
    (message `/Game/BP_Interface/BPI_Controls.TriggerSetStrafe` (`self.PlayerPawn`) ActionValue)))

(event `EnhancedInput|/Game/Input/IA_Rotation`
  (params (ActionValue :type "Float (double-precision)") (ElapsedSeconds :type "Float (double-precision)") (TriggeredSeconds :type "Float (double-precision)") (InputAction :type "InputAction Object Reference" :default "/Game/Input/IA_Rotation.IA_Rotation"))
  (:`Triggered`
    (message `/Game/BP_Interface/BPI_Controls.TriggerSetRotation` (`self.PlayerPawn`) ActionValue)))

(event `EnhancedInput|/Game/Input/IA_Action1`
  (params (ActionValue :type "Float (double-precision)") (ElapsedSeconds :type "Float (double-precision)") (TriggeredSeconds :type "Float (double-precision)") (InputAction :type "InputAction Object Reference" :default "/Game/Input/IA_Action1.IA_Action1"))
  (bind _playerpawn (`self.PlayerPawn`))
  (:`Triggered`
    (if (> TriggeredSeconds (/ (`GameplayStatics.GetWorldDeltaSeconds`) (`GameplayStatics.GetGlobalTimeDilation`)))
      (message `/Game/BP_Interface/BPI_Controls.TriggerSetAction1_hold` _playerpawn true)
      (else
        (message `/Game/BP_Interface/BPI_Controls.TriggerSetAction1_tap` _playerpawn false))))
  (:`Completed`
    (message `/Game/BP_Interface/BPI_Controls.TriggerSetAction1_hold` _playerpawn false)))

(event `EnhancedInput|/Game/Input/IA_Reloading`
  (params (ActionValue :type "Float (double-precision)") (ElapsedSeconds :type "Float (double-precision)") (TriggeredSeconds :type "Float (double-precision)") (InputAction :type "InputAction Object Reference" :default "/Game/Input/IA_Reloading.IA_Reloading"))
  (:`Triggered`
    (message `/Game/BP_Interface/BPI_Controls.TriggerReloading` (`self.PlayerPawn`))))

(event `Key|F1`
  (params (Key :type "Key Structure"))
  (:`Pressed`
    (bind _asbp_player (cast `/Game/BP_Player` (`self.PlayerPawn`)))
    (`/Game/BP_Player.SetLowGraphics` _asbp_player)))

(event `Key|F2`
  (params (Key :type "Key Structure"))
  (:`Pressed`
    (bind _asbp_player (cast `/Game/BP_Player` (`self.PlayerPawn`)))
    (`/Game/BP_Player.SetMediumGraphics` _asbp_player)))

(event `Key|F3`
  (params (Key :type "Key Structure"))
  (:`Pressed`
    (bind _asbp_player (cast `/Game/BP_Player` (`self.PlayerPawn`)))
    (`/Game/BP_Player.SetHighGraphics` _asbp_player)))

(fn `TriggerGetHUDInfo`
  (returns (Score :type "Float (double-precision)") (HP_current :type "Float (double-precision)") (HP_max :type "Float (double-precision)") (Ammo_Current :type Integer) (Ammo_Max :type Integer) (Ammo_Max_Laser :type "Float (double-precision)") (Weapon :type "/Game/Data/DataAsset/PDA_Weapon Object Reference") (ShootingType :type "/Game/Data/Enum/E_ShootingType Enum"))
  (return 0.0 0.0 0.0 0 0 0.0 null "NewEnumerator0"))

(fn `TriggerGetPlayer`
  (returns (Player :type "Actor Object Reference"))
  (return (`self.PlayerPawn`)))

(fn `UserConstructionScript`)