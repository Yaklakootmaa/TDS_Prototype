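; Enemy spawner that creates five named BP_Enemy variants on looping timers, the later four joining at staggered delays after BeginPlay.
; SpawnEnemy uses a per-type weighted roll to place each enemy at a random angle and range or at a reachable point near the player.
; ChangeSpawnDelay shortens each type's delay at growing game-time thresholds, but SpawnUpdateRate re-arms only the first timer.
; Tick prints game time and the first delay.
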(event `self.ReceiveTick`
  (params (DeltaSeconds :type "Float (single-precision)"))
  (`KismetSystemLibrary.PrintString` (`KismetStringLibrary.Concat_StrStr` (`KismetStringLibrary.Conv_DoubleToString` (`KismetSystemLibrary.GetGameTimeInSeconds`)) " /// " (`KismetStringLibrary.Conv_DoubleToString` (`self.SpawnDelay`))) true false (struct :`A` 1.0) 0.0))

(event `SpawnUpdateRate`
  (`KismetSystemLibrary.K2_SetTimerDelegate` (delegate `Spawn`) (`self.SpawnDelay`) true :!label _label))

(event `self.ReceiveBeginPlay`
  (bind _returnvalue (`GameplayStatics.GetActorOfClass` "/Game/BP_Player.BP_Player_C"))
  (set `self.PlayerRef` _returnvalue)
  (`|ExecutionSequence`
    (:`then_0`
      (goto _label))
    (:`then_1`
      (`KismetSystemLibrary.Delay` 10.0)
      (`KismetSystemLibrary.K2_SetTimerDelegate` (delegate `Spawn2`) (`self.SpawnDelay2`) true))
    (:`then_2`
      (`KismetSystemLibrary.Delay` 25.0)
      (`KismetSystemLibrary.K2_SetTimerDelegate` (delegate `Spawn3`) (`self.SpawnDelay3`) true))
    (:`then_3`
      (`KismetSystemLibrary.Delay` 40.0)
      (`KismetSystemLibrary.K2_SetTimerDelegate` (delegate `Spawn4`) (`self.SpawnDelay4`) true))
    (:`then_4`
      (`KismetSystemLibrary.Delay` 60.0)
      (`KismetSystemLibrary.K2_SetTimerDelegate` (delegate `Spawn5`) (`self.SpawnDelay5`) true))))

(event `Spawn`
  (`self.SpawnEnemy` (`self.EnemyName`) (`self.SpawnDelay`) 1.0)
  (bind (_spawndelayout _timesinceout) (`self.ChangeSpawnDelay` (`self.SpawnDelay`) (`self.TimeSinceGameStarted`))
    (:`Do`
      (set `self.SpawnDelay` _spawndelayout)
      (set `self.TimeSinceGameStarted` _timesinceout)
      (`self.SpawnUpdateRate`))))

(event `Spawn2`
  (`self.SpawnEnemy` "Enemy2" (`self.SpawnDelay2`) 0.8)
  (bind (_spawndelayout _timesinceout) (`self.ChangeSpawnDelay` (`self.SpawnDelay2`) (`self.TimeSinceGameStarted2`))
    (:`Do`
      (set `self.SpawnDelay2` _spawndelayout)
      (set `self.TimeSinceGameStarted2` _timesinceout)
      (`self.SpawnUpdateRate`))))

(event `Spawn3`
  (`self.SpawnEnemy` "Enemy3" (`self.SpawnDelay3`) 0.0)
  (bind (_spawndelayout _timesinceout) (`self.ChangeSpawnDelay` (`self.SpawnDelay3`) (`self.TimeSinceGameStarted3`) 1.15 1.15)
    (:`Do`
      (set `self.SpawnDelay3` _spawndelayout)
      (set `self.TimeSinceGameStarted3` _timesinceout)
      (`self.SpawnUpdateRate`))))

(event `Spawn4`
  (`self.SpawnEnemy` "Enemy4" (`self.SpawnDelay4`) 0.5)
  (bind (_spawndelayout _timesinceout) (`self.ChangeSpawnDelay` (`self.SpawnDelay4`) (`self.TimeSinceGameStarted4`) 1.15 1.15)
    (:`Do`
      (set `self.SpawnDelay4` _spawndelayout)
      (set `self.TimeSinceGameStarted4` _timesinceout)
      (`self.SpawnUpdateRate`))))

(event `Spawn5`
  (`self.SpawnEnemy` "Enemy5" (`self.SpawnDelay5`) 0.9)
  (bind (_spawndelayout _timesinceout) (`self.ChangeSpawnDelay` (`self.SpawnDelay5`) (`self.TimeSinceGameStarted5`) 1.05 1.05)
    (:`Do`
      (set `self.SpawnDelay5` _spawndelayout)
      (set `self.TimeSinceGameStarted5` _timesinceout)
      (`self.SpawnUpdateRate`))))

(fn `FindPositionAround`
  (params (IsAngleRandom :type Boolean) (IsRangeRandom :type Boolean) (Debug :type Boolean) (Range :type "Float (double-precision)") (AngleIncrement :type "Float (double-precision)") (UpdateTime :type "Float (double-precision)") (WeakSpawnChance :type "Float (double-precision)" :default 0.7))
  (returns (Position :type "Vector Structure"))
  (locals (Position_L :type "Vector Structure" :default (0.0 0.0 0.0)) (Range_L :type "Float (double-precision)" :default 0.0))
  (bind _returnvalue (`self.K2_GetActorLocation`))
  (bind _updatetime (`local.UpdateTime`))
  (if (`KismetMathLibrary.RandomBoolWithWeight` WeakSpawnChance)
    (if (`local.IsAngleRandom`)
      (set `self.SpawnAngle` (`KismetMathLibrary.RandomFloatInRange` 0.0 360.0))
      (else
        (set `self.SpawnAngle` (+ (`self.SpawnAngle`) (`local.AngleIncrement`)))))
    (if (`local.IsRangeRandom`)
      (set `local.Range_L` (`KismetMathLibrary.RandomFloatInRange` 50.0 (`local.Range`)))
      (else
        (set `local.Range_L` (`local.Range`))))
    (set `local.Position_L` (`KismetMathLibrary.RotateAngleAxis` (+ (`self.K2_GetActorLocation`) (* (`self.GetActorForwardVector`) (`local.Range_L`))) (`self.SpawnAngle`) (0.0 0.0 1.0)))
    (else
      (set `local.Position_L` (`NavigationSystemV1.K2_GetRandomReachablePointInRadius` (`self.K2_GetActorLocation` (`self.PlayerRef`)) (/ (`local.Range`) 3.0) null null))))
  (if (not (not (`local.Debug`)))
    (`KismetSystemLibrary.DrawDebugSphere` (`local.Position_L`) 50.0 12 (struct :`R` 1.0 :`B` 0.752942 :`A` 1.0) (`local.UpdateTime`) 2.0)
    (`KismetSystemLibrary.DrawDebugCircle` _returnvalue (`local.Range`) 96 (struct :`R` 1.0 :`G` 1.0 :`B` 1.0 :`A` 1.0) _updatetime 5.0 (1.0 0.0 0.0) (0.0 1.0 0.0))
    (`KismetSystemLibrary.DrawDebugCircle` _returnvalue (`local.Range_L`) 96 (struct :`R` 1.0 :`B` 0.751655 :`A` 1.0) _updatetime 5.0 (1.0 0.0 0.0) (0.0 1.0 0.0)))
  (return (`local.Position_L`)))

(fn `SpawnEnemy`
  (params (EnemyName :type Name) (UpdateTime :type "Float (double-precision)") (WeakSpawnChance :type "Float (double-precision)" :default 0.7))
  (bind _position (`self.FindPositionAround` true true false 2000.0 1.0 UpdateTime WeakSpawnChance))
  (bind _returnvalue (`AIBlueprintHelperLibrary.SpawnAIFromClass` "/Game/BP_Enemy.BP_Enemy_C" null _position (`KismetMathLibrary.FindLookAtRotation` (`self.K2_GetActorLocation`) (`self.K2_GetActorLocation` (`self.PlayerRef`))) false null))
  (bind _asbp_enemy (cast `/Game/BP_Enemy` _returnvalue))
  (set `/Game/BP_Enemy.EnemyName` EnemyName _asbp_enemy)
  (`/Game/BP_Enemy.SetEnemyParams` _asbp_enemy)
  (return))

(fn `UserConstructionScript`)