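; Projectile actor that deals direct or explosive damage and destroys itself on impact or five seconds after spawning.
; Non-explosive shots damage only on overlap, sending damage through the target's BPC_DamageSystem component.
; Explosive shots sphere-trace the radius, ignoring the owner, scale damage by a distance curve, then play a world camera shake.
; Optional debug drawing marks impacts and blast radius; GetOverlapActors is an uncalled BP_Enemy overlap query.
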(event `self.ReceiveBeginPlay`
  (set `self.Player` (`self.GetOwner`))
  (`SphereComponent.SetSphereRadius` (`self.ExplosionCollision`) (`self.ExplossionRadius`) true)
  (`KismetSystemLibrary.Delay` 5.0)
  (`self.K2_DestroyActor`))

(event `self.Cube.OnComponentBeginOverlap`
  (params (OverlappedComponent :type "PrimitiveComponent Object Reference") (OtherActor :type "Actor Object Reference") (OtherComp :type "PrimitiveComponent Object Reference") (OtherBodyIndex :type Integer) (bFromSweep :type Boolean) (SweepResult :type "HitResult Structure (by ref)"))
  (if (`self.IsExplosive`)
    (`self.ApplyDamageInRadius`
      (:`Completed`
        (`self.DoCameraShake`)))
    (else
      (`self.ApplyDamage` OtherActor false)
      (if (`self.Debug`)
        (`KismetSystemLibrary.DrawDebugPoint` (`self.K2_GetActorLocation`) 15.0 (struct :`R` 1.0 :`G` 0.129895 :`A` 1.0) 2.0))))
  (`self.K2_DestroyActor`))

(event `self.Cube.OnComponentHit`
  (params (HitComponent :type "PrimitiveComponent Object Reference") (OtherActor :type "Actor Object Reference") (OtherComp :type "PrimitiveComponent Object Reference") (NormalImpulse :type "Vector Structure") (Hit :type "HitResult Structure (by ref)"))
  (if (`self.Debug`)
    (`KismetSystemLibrary.DrawDebugPoint` (`self.K2_GetActorLocation`) 15.0 (struct :`R` 1.0 :`G` 0.129895 :`A` 1.0) 2.0))
  (if (`self.IsExplosive`)
    (`self.ApplyDamageInRadius`
      (:`Completed`
        (`self.DoCameraShake`))))
  (`self.K2_DestroyActor`))

(fn `UserConstructionScript`)