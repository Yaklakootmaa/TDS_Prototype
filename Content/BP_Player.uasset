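; Player pawn with simple move, strafe and rotate handlers and a weapon system configured from data assets, starting with the AR.
; SetWeapon copies the asset's stats, then a looping RPM timer or Tick (lasers, constant or pulsed) drives DoShot.
; DoShot spawns projectiles (single, burst, pellet) with ammo and reloads, or line-traces laser damage into BPC_DamageSystem.
; DoDispersion aims shots using random, curve-weighted, predefined-pattern or zero spread.
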(event Custom|Shoot
  (switch Utilities|FlowControl|Switch|SwitchonE_ShootingMode (Variables|Default|GetShootingMode)
    (:NewEnumerator1
      _)
    (:NewEnumerator2
      _))
  (if (Variables|Default|GetIsShootingOn)
    (CallFunction|DoShot false)))

(event Custom|BurstReloading
  (Variables|Ammo|SetIsBurstReloading true)
  (Utilities|FlowControl|Delay (Variables|Ammo|GetBurstReloadingTime))
  (if (> (- (Variables|Ammo|GetAmmoCurrent) (Variables|Ammo|GetAmmoBurstMax)) 0)
    (Variables|Ammo|SetAmmoCurrent (- (Variables|Ammo|GetAmmoCurrent) (Variables|Ammo|GetAmmoBurstMax)))
    (Variables|Ammo|SetAmmoBurstCurrent (Variables|Ammo|GetAmmoBurstMax))
    (else
      (Variables|Ammo|SetAmmoBurstCurrent (Variables|Ammo|GetAmmoCurrent))
      (Variables|Ammo|SetAmmoCurrent 0)))
  (Variables|Ammo|SetIsBurstReloading false))

(event Custom|SwitchToMG
  (Variables|Default|SetCurrentWeapon "/Game/Data/DA_WeaponMG.DA_WeaponMG")
  (Utilities|SetWeapon))

(event Custom|SwitchToShotgun
  (Variables|Default|SetCurrentWeapon "/Game/Data/DA_WeaponShotgun.DA_WeaponShotgun")
  (Utilities|SetWeapon))

(event Custom|ClipReloading
  (Variables|Ammo|SetIsClipReloading true)
  (Utilities|FlowControl|Delay (Variables|Ammo|GetClipReloadingTime))
  (Variables|Ammo|SetIsClipReloading false)
  (Variables|Ammo|SetAmmoCurrent (Variables|Ammo|GetAmmoMax)))

(event Custom|SwitchToLaser
  (Variables|Default|SetCurrentWeapon "/Game/Data/DA_WeaponLaser.DA_WeaponLaser")
  (Utilities|SetWeapon))

(event Custom|SwitchToPistol
  (Variables|Default|SetCurrentWeapon "/Game/Data/DA_WeaponPistol.DA_WeaponPistol")
  (Utilities|SetWeapon))

(event Custom|SwitchToSMG
  (Variables|Default|SetCurrentWeapon "/Game/Data/DA_WeaponSMG.DA_WeaponSMG")
  (Utilities|SetWeapon))

(event Custom|SwitchToAR
  (Variables|Default|SetCurrentWeapon "/Game/Data/DA_WeaponAR.DA_WeaponAR")
  (Utilities|SetWeapon))

(event EventBeginPlay
  (Utilities|FlowControl|Sequence
    (:then_0
      (Utilities|FlowControl|Sequence
        (:then_0
          (Utilities|FlowControl|Delay 5.0))
        (:then_1
          (CallFunction|SwitchtoAR))
        (:then_2
          (switch Utilities|FlowControl|Switch|SwitchonE_ShootingType (Variables|Default|GetShootingType)
            (:NewEnumerator3
              (Variables|Dispersion|SetDispersion%20Angle 1.5)
              (Variables|Dispersion|SetProjectileDistributionType "NewEnumerator1"))))))
    (:then_1
      (Class|BPIControls|TriggerGetPawnInfo(Message) (Game|GetPlayerController 0) self)
      (switch Utilities|FlowControl|Switch|SwitchonE_ShootingType (Variables|Default|GetShootingType)
        (:NewEnumerator0
          _)
        (:NewEnumerator1
          _)
        (:NewEnumerator2
          _))
      (Utilities|Time|SetTimerbyEvent (delegate Custom|Shoot) (|(1/(RF/60)) (Variables|Default|GetRPM)) true))))

(event EventTick
  (params (DeltaSeconds :type Float%20%28single-precision%29))
  (switch Utilities|FlowControl|Switch|SwitchonE_ShootingType (Variables|Default|GetShootingType)
    (:NewEnumerator0
      (Rendering|SetVisibility (Variables|Default|GetNS_LaserBeam) false false :!label _label))
    (:NewEnumerator1
      (goto _label))
    (:NewEnumerator2
      (goto _label))
    (:NewEnumerator3
      (if (Variables|Default|GetIsShootingOn)
        (Rendering|SetVisibility (Variables|Default|GetNS_LaserImpact) true true)
        (switch Utilities|FlowControl|Switch|SwitchonE_BeamType (Variables|Default|GetBeamType)
          (:NewEnumerator0
            _)
          (:NewEnumerator1
            (Utilities|FlowControl|Gate false :!label _label_2
              (:Exit
                (Utilities|FlowControl|Sequence
                  (:then_0
                    _)
                  (:then_1
                    (Utilities|FlowControl|DoOnce false :!label _label_3
                      (:Completed
                        (Utilities|FlowControl|Delay (Variables|Beam|GetBeamShootingTime))
                        (Utilities|FlowControl|Sequence
                          (:then_0
                            (Utilities|FlowControl|Sequence
                              (:then_0
                                (goto _label_2 Close))
                              (:then_1
                                (Rendering|SetVisibility (Variables|Default|GetNS_LaserImpact) false false)
                                (Utilities|FlowControl|Delay (Variables|Beam|GetBeamReloadingTime))
                                (goto _label_2 Open))))
                          (:then_1
                            (goto _label_3 Reset)))))))))))
        (CallFunction|Shoot)
        (else
          (goto _label))))
    (:NewEnumerator4
      (goto _label))
    (:NewEnumerator5
      (goto _label))))

(event EventTriggerSetMovement
  (params (Axis :type Float%20%28double-precision%29))
  (Transformation|AddActorWorldOffset (* (Transformation|GetActorForwardVector) (* Axis 1e+01))))

(event EventTriggerSetRotation
  (params (Axis :type Float%20%28double-precision%29))
  (Class|Actor|AddActorWorldRotation (* "0.000000,1.000000,0.000000" (* Axis 1.0))))

(event EventTriggerSetStrafe
  (params (Axis :type Float%20%28double-precision%29))
  (Transformation|AddActorWorldOffset (* (Transformation|GetActorRightVector) (* Axis 1e+01))))

(event EventTriggerSetAction1Tap
  (params (IsHolding :type Boolean))
  (Variables|Default|SetIsShootingOn IsHolding)
  (switch Utilities|FlowControl|Switch|SwitchonE_ShootingType (Variables|Default|GetShootingType)
    (:NewEnumerator0
      _)
    (:NewEnumerator1
      _)
    (:NewEnumerator2
      _))
  (switch Utilities|FlowControl|Switch|SwitchonE_ShootingMode (Variables|Default|GetShootingMode)
    (:NewEnumerator0
      _)
    (:NewEnumerator2
      _))
  (Utilities|FlowControl|DoOnce false :!label _label
    (:Completed
      (CallFunction|DoShot false)
      (Utilities|FlowControl|Delay (/ (|(1/(RF/60)) (Variables|Default|GetRPM)) 2.0))
      (goto _label Reset))))

(event EventTriggerSetAction1Hold
  (params (IsHolding :type Boolean))
  (Variables|Default|SetIsShootingOn IsHolding))

(fn ConstructionScript)

(fn DoCameraShake
  (params (Shake :type Camera%20Shake%20Base%20Class%20Reference))
  (Camera|PlayWorldCameraShake Shake (Transformation|GetWorldLocation (Variables|Default|GetCamera)) 0.0 5e+02)
  (return))

(fn DoShot
  (params (ShowDebug :type Boolean))
  (bind _dispersion_angle (Variables|Dispersion|GetDispersion%20Angle))
  (bind _dispersionpattern (Variables|Dispersion|GetDispersionPattern))
  (bind _dispersioncurve (Variables|Dispersion|GetDispersionCurve))
  (bind _ns_laserbeam (Variables|Default|GetNS_LaserBeam))
  (bind (_projectiledirection _startlocation _endloctaion) (Dispersion|DoDispersion _dispersion_angle _dispersioncurve _dispersionpattern ShowDebug))
  (if (Math|Boolean|NANDBoolean (Variables|Ammo|GetIsClipReloading) (Variables|Ammo|GetIsBurstReloading))
    (switch Utilities|FlowControl|Switch|SwitchonE_ShootingType (Variables|Default|GetShootingType)
      (:NewEnumerator0
        _)
      (:NewEnumerator1
        _)
      (:NewEnumerator2
        _)
      (:NewEnumerator3
        (bind _output_get (LocalVariables|SetStartLocation_L _startlocation))
        (bind _output_get_2 (LocalVariables|SetEndLocation_L _endloctaion))
        (bind _outhit (Collision|LineTraceByChannel _output_get _output_get_2 "TraceTypeQuery1" false 0 "None" true "(R=1.000000,G=0.000000,B=0.000000,A=1.000000)" "(R=0.000000,G=1.000000,B=0.000000,A=1.000000)" 1.0))
        (LocalVariables|SetLaserImpactLocation_L (.location _outhit))
        (Rendering|SetVisibility _ns_laserbeam true false)
        (Effects|Components|ParticleSystem|SetColorParameter _ns_laserbeam "Colour" "(R=0.000000,G=1.000000,B=0.804625,A=1.000000)")
        (Effects|Components|ParticleSystem|SetVectorParameter _ns_laserbeam "LaserEnd" (select (.bblockinghit _outhit) (.location _outhit) "0, 0, 0"))
        (Transformation|SetWorldLocation (Variables|Default|GetNS_LaserImpact) (.location _outhit) false false)
        (CallFunction|DoCameraShake (Variables|Default|GetCameraShake))
        (Utilities|IsValid (.hitactor _outhit)
          (:Is%20Valid
            (Utilities|IsValid (Actor|GetComponentbyClass (.hitactor _outhit) "/Game/Component/BPC_DamageSystem.BPC_DamageSystem_C")
              (:Is%20Valid
                (Class|BPIGameSystems|TriggerCauseDamage(Message) (Actor|GetComponentbyClass (.hitactor _outhit) "/Game/Component/BPC_DamageSystem.BPC_DamageSystem_C") (* (Variables|Default|GetDamagePerSecond) (Utilities|Time|GetWorldDeltaSeconds)))
                (return))
              (:Is%20Not%20Valid
                (return))))
          (:Is%20Not%20Valid
            (return)))))
    (switch Utilities|FlowControl|Switch|SwitchonE_ShootingMethod (Variables|Default|GetShootingMethod)
      (:NewEnumerator0
        (if (> (Variables|Ammo|GetAmmoCurrent) 0)
          (bind _result (Math|Integer|DecrementInt (Variables|Ammo|GetAmmoCurrent))
            (:%20%20
              (Variables|Ammo|SetAmmoCurrent _result)
              (bind _output_get_3 (LocalVariables|SetProjectileTransform_L (.ProjectileDirection (Dispersion|DoDispersion (Variables|Dispersion|GetDispersion%20Angle) (Variables|Dispersion|GetDispersionCurve) (Variables|Dispersion|GetDispersionPattern) ShowDebug)) :!label _label))
              (Game|SpawnActorfromClass "/Game/BP_Projectile.BP_Projectile_C" _output_get_3 "Undefined" 0 (Variables|Default|GetDamagePerProjectile) 0)
              (CallFunction|DoCameraShake (Variables|Default|GetCameraShake))
              (return)))
          (else
            (CallFunction|ClipReloading))))
      (:NewEnumerator2
        (bind _result_2 (Math|Integer|DecrementInt (Variables|Ammo|GetAmmoBurstCurrent))
          (:%20%20
            (bind _output_get_4 (Variables|Ammo|SetAmmoBurstCurrent _result_2))
            (if (> _output_get_4 -1)
              (goto _label)
              (elif (> (Variables|Ammo|GetAmmoCurrent) 0)
                (CallFunction|BurstReloading)
                (else
                  (CallFunction|ClipReloading)))))))
      (:NewEnumerator1
        (if (> (Variables|Ammo|GetAmmoCurrent) 0)
          (bind _result_3 (Math|Integer|DecrementInt (Variables|Ammo|GetAmmoCurrent))
            (:%20%20
              (Variables|Ammo|SetAmmoCurrent _result_3)
              (for _index (range 1 (Variables|Ammo|GetAmmoPelletMax))
                (bind _output_get_5 (LocalVariables|SetProjectileTransform_L (.ProjectileDirection (Dispersion|DoDispersion (Variables|Dispersion|GetDispersion%20Angle) (Variables|Dispersion|GetDispersionCurve) (Variables|Dispersion|GetDispersionPattern) ShowDebug))))
                (Game|SpawnActorfromClass "/Game/BP_Projectile.BP_Projectile_C" _output_get_5 "Undefined" 0 (Variables|Default|GetDamagePerProjectile) 0))
              (CallFunction|DoCameraShake (Variables|Default|GetCameraShake))))
          (else
            (CallFunction|ClipReloading)))
        (return)))
    (return)
    (else
      (return))))

(fn DoDispersion
  (params (DispersionAngle :type Float%20%28double-precision%29) (DispersionCurve :type Curve%20Float%20Object%20Reference) (PredefinedAnglesArray :type Array%20of%20Rotators) (ShowDebug :type Boolean))
  (bind _arrow (Variables|Default|GetArrow))
  (bind _arrow_2 (Variables|Default|GetArrow))
  (bind _arrow_3 (Variables|Default|GetArrow))
  (bind _returnvalue (Transformation|GetWorldLocation _arrow))
  (bind _returnvalue_2 (Transformation|GetWorldLocation _arrow_3))
  (LocalVariables|SetPredefinedAngles_L PredefinedAnglesArray)
  (LocalVariables|SetRadiusMax_L (* (Math|Trig|Tan(Degrees) DispersionAngle) (LocalVariables|GetProjectileDistance_L)))
  (LocalVariables|SetRandomAngle_L (Math|Random|RandomFloatinRange 0.0 3.6e+02))
  (switch Utilities|FlowControl|Switch|SwitchonE_ProjectileDistributionType (Variables|Dispersion|GetProjectileDistributionType)
    (:NewEnumerator0
      (bind _output (Dispersion|RandomPointinCircle (LocalVariables|GetRadiusMax_L) DispersionCurve false))
      (LocalVariables|SetRandomXY-Offest_L _output))
    (:NewEnumerator1
      (bind _output_2 (Dispersion|RandomPointinCircle (LocalVariables|GetRadiusMax_L) DispersionCurve true :!label _label))
      (LocalVariables|SetRandomXY-Offest_L _output_2))
    (:NewEnumerator2
      (if (not (Utilities|Array|IsNotEmpty (LocalVariables|GetPredefinedAngles_L)))
        (goto _label)
        (else
          (if (!= (+ (Variables|Dispersion|GetDPA_Index) 1) (Utilities|Array|Length (LocalVariables|GetPredefinedAngles_L)))
            _
            (else
              (bind _output_get (Variables|Dispersion|SetDPA_Index -1))))
          (bind _result (Math|Integer|IncrementInt _output_get)
            (:%20%20
              (bind _output_get_2 (LocalVariables|SetStart_L (Transformation|GetWorldLocation _arrow_2)))
              (LocalVariables|SetEnd_L (+ _output_get_2 (* (Math|Vector|GetForwardVector (Math|Rotator|CombineRotators (Transformation|GetWorldRotation _arrow_2) (* (Utilities|Array|Get(acopy) (LocalVariables|GetPredefinedAngles_L) _result) DispersionAngle))) (LocalVariables|GetProjectileDistance_L))))
              (if ShowDebug
                (Dispersion|DispersionDebug (LocalVariables|GetStart_L) (LocalVariables|GetEnd_L)))
              (return (Math|Transform|MakeTransform _output_get_2 (Math|Rotator|CombineRotators (Transformation|GetWorldRotation _arrow_2) (* (Utilities|Array|Get(acopy) (LocalVariables|GetPredefinedAngles_L) _result) DispersionAngle)) (Variables|Default|GetProjectileScale)) (LocalVariables|GetStart_L) (LocalVariables|GetEnd_L)))))))
    (:NewEnumerator3
      (LocalVariables|SetStart_L _returnvalue)
      (LocalVariables|SetEnd_L (+ (Transformation|GetWorldLocation _arrow) (* (Math|Vector|GetForwardVector _arrow) (LocalVariables|GetProjectileDistance_L))))
      (if ShowDebug
        (Dispersion|DispersionDebug (LocalVariables|GetStart_L) (LocalVariables|GetEnd_L)))
      (return (Math|Transform|MakeTransform _returnvalue (Transformation|GetWorldRotation _arrow) (Variables|Default|GetProjectileScale)) (LocalVariables|GetStart_L) (LocalVariables|GetEnd_L))))
  (LocalVariables|SetStart_L _returnvalue_2)
  (LocalVariables|SetEnd_L (+ (+ _returnvalue_2 (* (Math|Vector|GetForwardVector _arrow_3) (LocalVariables|GetProjectileDistance_L))) (* (Math|Vector|GetRightVector _arrow_3) (.X (Math|Vector2D|BreakVector2D (LocalVariables|GetRandomXY-Offest_L)))) (* (Math|Vector|GetUpVector _arrow_3) (.Y (Math|Vector2D|BreakVector2D (LocalVariables|GetRandomXY-Offest_L))))))
  (if ShowDebug
    (Dispersion|DispersionDebug (LocalVariables|GetStart_L) (LocalVariables|GetEnd_L)))
  (return (Math|Transform|MakeTransform (LocalVariables|GetStart_L) (Math|Rotator|MakeRotator 0.0 0.0 (.yaw (Math|Rotator|FindLookatRotation (LocalVariables|GetStart_L) (LocalVariables|GetEnd_L)))) (Variables|Default|GetProjectileScale)) (LocalVariables|GetStart_L) (LocalVariables|GetEnd_L)))

(fn RandomPointinCircle
  (params (Radius :type Float%20%28double-precision%29) (Curve :type Curve%20Float%20Object%20Reference) (IsCurveBased :type Boolean))
  (LocalVariables|SetAngle (Math|Random|RandomFloatinRange 0.0 3.6e+02))
  (if IsCurveBased
    (Utilities|IsValid Curve
      (:Is%20Valid
        (LocalVariables|SetDistanceFromCenter (Math|Random|RandomFloatinRange 0.0 (* Radius (Math|Curves|GetFloatValue Curve (Math|Random|RandomFloatinRange 0.0 1.0))))))
      (:Is%20Not%20Valid
        (LocalVariables|SetDistanceFromCenter (Math|Random|RandomFloatinRange 0.0 Radius) :!label _label)))
    (else
      (goto _label)))
  (return (Math|Vector2D|MakeVector2D (* (LocalVariables|GetDistanceFromCenter) (Math|Trig|Cos(Degrees) (LocalVariables|GetAngle))) (* (LocalVariables|GetDistanceFromCenter) (Math|Trig|Sin(Degrees) (LocalVariables|GetAngle))))))

(fn DispersionDebug
  (params (Start :type Vector) (End :type Vector))
  (bind (_x _y) (Class|KismetMathLibrary|BreakVector3f Start))
  (bind (_x_2 _y_2) (Class|KismetMathLibrary|BreakVector3f End))
  (bind _arrow (Variables|Default|GetArrow))
  (bind _returnvalue (Transformation|GetWorldLocation _arrow))
  (Collision|LineTraceByChannel (Math|Vector|MakeVector _x _y (.z _returnvalue)) (Math|Vector|MakeVector _x_2 _y_2 (.z _returnvalue)) "TraceTypeQuery1" false 0 "ForDuration" true "(R=1.000000,G=0.000000,B=0.000000,A=1.000000)" "(R=0.000000,G=1.000000,B=0.000000,A=1.000000)" 2.0)
  (return))