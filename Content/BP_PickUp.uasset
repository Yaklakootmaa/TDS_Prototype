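; BP_PickUp is a pickup actor that grants either a weapon or a power-up, such as Health, Freeze or Nuke.
; Every Tick it draws a debug string at its location naming the weapon or power-up.
; When any actor overlaps its Sphere, it sends that actor TriggerPickUpMessage with the pickup type, weapon and power-up, then destroys itself.
; BeginPlay caches the first BP_Player in Pawn, which the graph never reads.
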(event `self.ReceiveBeginPlay`
  (bind _outactors (`GameplayStatics.GetAllActorsOfClass` "/Game/BP_Player.BP_Player_C"))
  (set `self.Pawn` (`|GetArrayItem` _outactors)))

(event `self.ReceiveTick`
  (params (DeltaSeconds :type "Float (single-precision)"))
  (switch `/Game/Enum/E_PickUpType` (`self.PickUpType`)
    (:`NewEnumerator0`
      (set `self.Text` (`KismetSystemLibrary.GetDisplayName` (`self.Weapon`))))
    (:`NewEnumerator1`
      (switch `/Game/Enum/E_PowerUp` (`self.PowerUp`)
        (:`NewEnumerator0`
          (set `self.Text` "Health"))
        (:`NewEnumerator1`
          (set `self.Text` "SpeedUp"))
        (:`NewEnumerator2`
          (set `self.Text` "Freeze"))
        (:`NewEnumerator3`
          (set `self.Text` "BulletTime"))
        (:`NewEnumerator4`
          (set `self.Text` "Nuke"))
        (:`NewEnumerator5`
          (set `self.Text` "X3"))
        (:`NewEnumerator7`
          (set `self.Text` "Immortality")))))
  (`KismetSystemLibrary.DrawDebugString` (`self.K2_GetActorLocation`) (`self.Text`) null (struct :`A` 1.0)))

(event `self.Sphere.OnComponentBeginOverlap`
  (params (OverlappedComponent :type "PrimitiveComponent Object Reference") (OtherActor :type "Actor Object Reference") (OtherComp :type "PrimitiveComponent Object Reference") (OtherBodyIndex :type Integer) (bFromSweep :type Boolean) (SweepResult :type "HitResult Structure (by ref)"))
  (message `/Game/BP_Interface/BPI_GameSystems.TriggerPickUp` OtherActor (`self.PickUpType`) (`self.Weapon`) (`self.PowerUp`))
  (`self.K2_DestroyActor`))

(fn `UserConstructionScript`)